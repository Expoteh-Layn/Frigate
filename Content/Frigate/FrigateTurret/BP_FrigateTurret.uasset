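; Frigate turret actor that aims at a settable target actor, optionally assigned as an initial target during construction.
; A delegate turret manipulator, initialized with a rotator interpolator, receives the target's root component and drives aiming through bound events.
; Those events apply pitch and yaw rotations to a turret wrapper child actor and feed its current world transforms back to the manipulator.
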(event Custom|SetTurretRotations_Event
  (params (PitchRotation :type Rotator) (YawRotation :type Rotator) (PitchLocalRotation :type Float%20%28double-precision%29) (PitchLocalOffset :type Float%20%28double-precision%29) (YawLocalOffset :type Float%20%28double-precision%29))
  (Default|SetTurretRotation (Variables|Default|GetTurretWrapper) PitchRotation YawRotation))

(event Custom|UpdateCurrentRotations_Event
  (bind _turretwrapper (Variables|Default|GetTurretWrapper))
  (bind (_pitchworldtransform _yawworldtransform) (Default|GetTurretWorldTransform _turretwrapper))
  (bind (_location _rotation) (Math|Transform|BreakTransform _yawworldtransform))
  (bind (_location_2 _rotation_2) (Math|Transform|BreakTransform _pitchworldtransform))
  (Default|UpdateTurretCurrentValues (Variables|Default|GetBP_DelegateTurretManipulator) _location_2 _rotation_2 _location _rotation))

(event EventBeginPlay
  (bind _bp_delegateturretmanipulator (Variables|Default|GetBP_DelegateTurretManipulator))
  (EventDispatchers|AssignSetTurretRotations _bp_delegateturretmanipulator (delegate Custom|SetTurretRotations_Event))
  (EventDispatchers|AssignUpdateTurretCurrentRotations _bp_delegateturretmanipulator (delegate Custom|UpdateCurrentRotations_Event)))

(fn ConstructionScript
  (bind _initialtarget (Variables|Default|GetInitialTarget))
  (bind _asbp_frigate_turret_wrapper (Utilities|Casting|CastToBP_FrigateTurretWrapper (Variables|/Script/Engine.ChildActorComponent|GetChildActor (Variables|Default|GetTurretWrapperChildComponent))))
  (Variables|Default|SetTurretWrapper _asbp_frigate_turret_wrapper)
  (Default|Init (Variables|Default|GetBP_DelegateTurretManipulator) (Variables|Default|GetBP_InterpRotatorInterpolator))
  (Utilities|IsValid _initialtarget
    (:Is%20Valid
      (CallFunction|SetTarget _initialtarget))))

(fn SetTarget
  (params (Target :type Actor%20Object%20Reference))
  (bind _bp_delegateturretmanipulator (Variables|Default|GetBP_DelegateTurretManipulator))
  (Utilities|IsValid Target
    (:Is%20Valid
      (Default|SetTarget _bp_delegateturretmanipulator (Variables|/Script/Engine.Actor|GetRootComponent Target)))
    (:Is%20Not%20Valid
      (Default|SetTarget _bp_delegateturretmanipulator))))

(fn ClearTarget
  (Default|ClearTarget (Variables|Default|GetBP_DelegateTurretManipulator)))