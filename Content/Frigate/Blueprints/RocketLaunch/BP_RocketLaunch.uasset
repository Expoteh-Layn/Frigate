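; BP_RocketLaunch is a rocket launcher assembly that pairs a door with an animated rocket, both held as child actors.
; BeginPlay caches both child actors and binds to the door's opened event.
; Launch opens the door if closed; once it has opened, the rocket starts and detaches, keeping its world transform.
; Duplicate spawns and returns a new launcher at the same transform.
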(event Custom|DoorOpenned_Event
  (Default|Start (Variables|Default|GetRocketWithAnim))
  (Transformation|DetachFromComponent (Variables|Default|GetCAC_RocketWithAnimation) "KeepWorld" "KeepWorld" "KeepWorld" true))

(event EventBeginPlay
  (Private|Unwrap)
  (EventDispatchers|AssignDoorOpenned (Variables|Default|GetRocketDoor) (delegate Custom|DoorOpenned_Event)))

(fn ConstructionScript)

(fn Launch
  (if (Default|IsClosed (Variables|Default|GetRocketDoor))
    (Default|SetOpen (Variables|Default|GetRocketDoor) true)))

(fn Unwrap
  (Utilities|FlowControl|Sequence
    (:then_0
      (bind _asbp_rocket_door (Utilities|Casting|CastToBP_RocketDoor (Variables|/Script/Engine.ChildActorComponent|GetChildActor (Variables|Default|GetCAC_RocketDoor))))
      (Variables|Default|SetRocketDoor _asbp_rocket_door))
    (:then_1
      (bind _asbp_rocket_with_animation (Utilities|Casting|CastToBP_RocketWithAnimation (Variables|/Script/Engine.ChildActorComponent|GetChildActor (Variables|Default|GetCAC_RocketWithAnimation))))
      (Variables|Default|SetRocketWithAnim _asbp_rocket_with_animation))))

(fn Duplicate
  (bind _returnvalue (Game|SpawnActorfromClass "BP_RocketLaunch_C" (Transformation|GetActorTransform) "Undefined" "MultiplyWithRoot" 0 0))
  (return _returnvalue))