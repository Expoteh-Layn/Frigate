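; BP_RocketDeploy is a rocket deploy unit on the frigate that cycles a rocket door when launched.
; On BeginPlay it casts its child actor component to BP_RocketDoor, caches the reference and binds to the door's opened event.
; Launch opens the door only if it is closed, and the opened event immediately sets it closed again.
; No rocket spawning happens in these graphs.
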(event Custom|DoorOpenned_Event
  (Default|SetOpen (Variables|Default|GetRocketDoor) false))

(event EventBeginPlay
  (Private|Unwrap)
  (EventDispatchers|AssignDoorOpenned (Variables|Default|GetRocketDoor) (delegate Custom|DoorOpenned_Event)))

(fn ConstructionScript)

(fn Launch
  (if (Default|IsClosed (Variables|Default|GetRocketDoor))
    (Default|SetOpen (Variables|Default|GetRocketDoor) true)))

(fn Unwrap
  (Utilities|FlowControl|Sequence
    (:then_0
      (bind _asbp_rocket_door (Utilities|Casting|CastToBP_RocketDoor (Variables|/Script/Engine.ChildActorComponent|GetChildActor (Variables|Default|GetCAC_RocketDoor))))
      (Variables|Default|SetRocketDoor _asbp_rocket_door))))