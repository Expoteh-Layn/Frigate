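; BP_Frigate is a frigate that delegates movement to a movement component and carries two turrets and a rocket door as child actors.
; On BeginPlay it casts the child actors into typed references, initializes movement, and assigns each turret its own target.
; It exposes pass-through functions for movement input and speed multipliers, a getter for both turrets, and a call to open or close the rocket door.
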(event EventBeginPlay
  (Private|Unwrap)
  (Default|Init (Variables|Default|GetBP_FrigateMovement) (Variables|Default|GetFrigate))
  (Default|SetTarget (Variables|Default|GetLeftTurret) (Variables|Initial|GetLeftTurretTarget))
  (Default|SetTarget (Variables|Default|GetRightTurret) (Variables|Initial|GetRightTurretTarget)))

(fn ConstructionScript)

(fn MoveForward
  (params (value :type Float%20%28double-precision%29))
  (Default|MoveForward (Variables|Default|GetBP_FrigateMovement) value))

(fn MoveRight
  (params (Value :type Float%20%28double-precision%29))
  (Default|MoveRight (Variables|Default|GetBP_FrigateMovement) Value))

(fn SetForwardSpeedMulti
  (params (value :type Float%20%28double-precision%29))
  (Default|SetForwardSpeedMulti (Variables|Default|GetBP_FrigateMovement) value))

(fn SetRightSpeedMulti
  (params (value :type Float%20%28double-precision%29))
  (Default|SetRightSpeedMulti (Variables|Default|GetBP_FrigateMovement) value))

(fn Unwrap
  (Utilities|FlowControl|Sequence
    (:then_0
      (bind _asbp_frigate_turret (Utilities|Casting|CastToBP_FrigateTurret (Variables|/Script/Engine.ChildActorComponent|GetChildActor (Variables|Default|GetCAC_LeftTurret))))
      (Variables|Default|SetLeftTurret _asbp_frigate_turret))
    (:then_1
      (bind _asbp_frigate_turret_2 (Utilities|Casting|CastToBP_FrigateTurret (Variables|/Script/Engine.ChildActorComponent|GetChildActor (Variables|Default|GetCAC_RightTurret))))
      (Variables|Default|SetRightTurret _asbp_frigate_turret_2))
    (:then_2
      (bind _asbp_rocket_door (Utilities|Casting|CastToBP_RocketDoor (Variables|/Script/Engine.ChildActorComponent|GetChildActor (Variables|Default|GetCAC_RocketDoor1))))
      (Variables|Default|SetRocketDoor1 _asbp_rocket_door))))

(fn GetTurrets
  (return (Variables|Default|GetLeftTurret) (Variables|Default|GetRightTurret)))

(fn OpenRocketDoor
  (params (Openned :type Boolean))
  (Default|SetOpen (Variables|Default|GetRocketDoor1) Openned))