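; Player pawn for controlling a frigate, forwarding input to a BP_Frigate child actor and a BPPlayerCamera helper.
; BeginPlay unwraps the child actor, sets its speed multipliers and turret targets, configures camera zoom and attaches the spring arm to the frigate.
; Movement axes forward only full ±1 input, with a separate Stop action sending zero.
; Camera axes drive orbit and delta-time-scaled zoom, while weapon actions toggle each turret's firing.
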(event EventBeginPlay
  (Private|Unwrap)
  (Private|InitFrigate)
  (Private|InitPlayerCamera))

(event Input|ActionEvents|InputActionLeftWeaponGun
  (params (Key :type Key%20Structure :default "None"))
  (bind _frigate (Variables|Default|GetFrigate))
  (bind _leftturret (Default|GetTurrets _frigate))
  (:Pressed
    (Default|SetShoot _leftturret (not (Default|IsShoot _leftturret)))))

(event Input|ActionEvents|InputActionRightWeaponGun
  (params (Key :type Key%20Structure :default "None"))
  (bind _frigate (Variables|Default|GetFrigate))
  (bind _rightturret (Default|GetTurrets _frigate))
  (:Pressed
    (Default|SetShoot _rightturret (not (Default|IsShoot _rightturret)))))

(event Input|ActionEvents|InputActionStop
  (params (Key :type Key%20Structure :default "None"))
  (:Pressed
    (Default|MoveRight (Variables|Default|GetFrigate) 0.0)
    (Default|MoveForward (Variables|Default|GetFrigate) 0.0)))

(event Input|AxisEvents|InputAxisMoveForward
  (params (AxisValue :type Float%20%28single-precision%29))
  (bind _frigate (Variables|Default|GetFrigate))
  (Utilities|FlowControl|Sequence
    (:then_0
      (if (CallFunction|NearlyEq AxisValue 1.0)
        (Default|MoveForward _frigate AxisValue)))
    (:then_1
      (if (CallFunction|NearlyEq AxisValue -1.0)
        (Default|MoveForward _frigate AxisValue)))))

(event Input|AxisEvents|InputAxisMoveRight
  (params (AxisValue :type Float%20%28single-precision%29))
  (bind _frigate (Variables|Default|GetFrigate))
  (Utilities|FlowControl|Sequence
    (:then_0
      (if (CallFunction|NearlyEq AxisValue 1.0)
        (Default|MoveRight _frigate AxisValue)))
    (:then_1
      (if (CallFunction|NearlyEq AxisValue -1.0)
        (Default|MoveRight _frigate AxisValue)))))

(event Input|AxisEvents|InputAxisCameraUp
  (params (AxisValue :type Float%20%28single-precision%29))
  (Default|AddUp (Variables|Default|GetBP_PlayerCamera) AxisValue))

(event Input|AxisEvents|InputAxisCameraRight
  (params (AxisValue :type Float%20%28single-precision%29))
  (Default|AddRight (Variables|Default|GetBP_PlayerCamera) AxisValue))

(event Input|AxisEvents|InputAxisCameraZoom
  (params (AxisValue :type Float%20%28single-precision%29))
  (Default|AddLength (Variables|Default|GetBP_PlayerCamera) (* AxisValue (Variables|Default|GetZoomSpeedCore) (Utilities|Time|GetWorldDeltaSeconds) (Variables|Initial|GetZoomSpeed))))

(fn ConstructionScript)

(fn Unwrap
  (Utilities|FlowControl|Sequence
    (:then_0
      (bind _asbp_frigate (Utilities|Casting|CastToBP_Frigate (Variables|/Script/Engine.ChildActorComponent|GetChildActor (Variables|Default|GetCAC_Frigate))))
      (Variables|Default|SetFrigate _asbp_frigate))))

(fn InitFrigate
  (bind _frigate (Variables|Default|GetFrigate))
  (bind (_leftturret _rightturret) (Default|GetTurrets _frigate))
  (Default|SetForwardSpeedMulti _frigate (Variables|Initial|GetFrigateForwardSpeed))
  (Default|SetRightSpeedMulti _frigate (Variables|Initial|GetFrigateRightSpeed))
  (Default|SetTarget _leftturret (Variables|Initial|GetLeftTurretTarget))
  (Default|SetTarget _rightturret (Variables|Initial|GetRightTurretTarget)))

(fn InitPlayerCamera
  (bind _bp_playercamera (Variables|Default|GetBP_PlayerCamera))
  (Default|SetCamera _bp_playercamera (Variables|Default|GetCamera1))
  (Default|SetSpringArm _bp_playercamera (Variables|Default|GetSpringArm))
  (Default|SetLengthRange (Variables|Default|GetBP_PlayerCamera) (Variables|Initial|GetMinZoom) (Variables|Initial|GetMaxZoom))
  (Default|SetLength (Variables|Default|GetBP_PlayerCamera) (Variables|Default|GetInitialZoom))
  (Transformation|AttachComponentToComponent (Variables|Default|GetSpringArm) (Variables|/Script/Engine.Actor|GetRootComponent (Variables|Default|GetFrigate)) "None" "KeepWorld" "KeepWorld" "KeepWorld" true))

(fn NearlyEq
  (params (Input :type Float%20%28double-precision%29) (NearlyEq :type Float%20%28double-precision%29))
  (return (Math|Float|NearlyEqual(Float) Input NearlyEq 0.01)))