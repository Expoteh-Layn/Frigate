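; BP_PlayerCamera controls a player camera through a Camera and Spring Arm handed to it by setters.
; Zoom sets or adds to the arm length, clamped to a configurable range.
; AddUp applies local pitch through a MathHelper fetched on BeginPlay and clamps it to pitch limits, while AddRight adds world-space yaw to the arm.
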(event EventBeginPlay
  (bind _instance (Utilities|GetorCreateMathHelper))
  (Variables|Components|SetMathHelper _instance))

(event EventTick
  (params (DeltaSeconds :type Float%20%28single-precision%29)))

(fn SetCamera
  (params (Camera :type Camera%20Component%20Object%20Reference))
  (Variables|Default|SetCamera Camera))

(fn SetSpringArm
  (params (SpringArm :type Spring%20Arm%20Component%20Object%20Reference))
  (Utilities|FlowControl|Sequence
    (:then_0
      (Utilities|IsValid (Variables|Default|GetSpringArm)
        (:Is%20Valid
          (Variables|/Script/Engine.SpringArmComponent|SetTargetArmLength SpringArm (Variables|/Script/Engine.SpringArmComponent|GetTargetArmLength (Variables|Default|GetSpringArm))))))
    (:then_1
      (Variables|Default|SetSpringArm SpringArm))))

(fn SetLengthRange
  (params (MinLength :type Float%20%28double-precision%29) (MaxLength :type Float%20%28double-precision%29))
  (Variables|Initial|SetLengthClamp (Math|Vector2D|MakeVector2D MinLength MaxLength)))

(fn SetLength
  (params (Value :type Float%20%28double-precision%29))
  (bind _lengthclamp (Variables|Initial|GetLengthClamp))
  (Variables|/Script/Engine.SpringArmComponent|SetTargetArmLength (Variables|Default|GetSpringArm) (Math|Float|Clamp(Float) Value (.x _lengthclamp) (.y _lengthclamp))))

(fn AddLength
  (params (Value :type Float%20%28double-precision%29))
  (CallFunction|SetLength (+ (Variables|/Script/Engine.SpringArmComponent|GetTargetArmLength (Variables|Default|GetSpringArm)) Value)))

(fn AddUp
  (params (Value :type Float%20%28double-precision%29))
  (bind _returnvalue (Math|Rotator|MakeRotator 0.0 Value 0.0))
  (bind _springarm (Variables|Default|GetSpringArm))
  (bind _mathhelper (Variables|Components|GetMathHelper))
  (bind _pitchclamp (Variables|Initial|GetPitchClamp))
  (bind _returnvalue_2 (Transformation|GetWorldRotation _springarm))
  (bind _output (Default|AddLocalRotation _mathhelper _returnvalue_2 _returnvalue))
  (bind (_roll _pitch _yaw) (Math|Rotator|BreakRotator _output))
  (Transformation|SetWorldRotation _springarm (Math|Rotator|MakeRotator _roll (Math|Float|Clamp(Float) _pitch (.x _pitchclamp) (.y _pitchclamp)) _yaw) false false))

(fn AddRight
  (params (Value :type Float%20%28double-precision%29))
  (Transformation|AddWorldRotation (Variables|Default|GetSpringArm) (Math|Rotator|MakeRotator 0.0 0.0 Value) false false))