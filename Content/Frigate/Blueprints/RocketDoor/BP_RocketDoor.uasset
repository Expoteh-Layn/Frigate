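; BP_RocketDoor is a rocket door in the Frigate content that swings open and closed by pitch rotation.
; SetOpen tells the BPDoorStopwatch to count to OpenTime to open, or to zero to close.
; Each stopwatch update sets the root's relative pitch to the elapsed fraction of OpenTime times RotateAngle.
; The construction script applies the configurable Mesh to the static mesh component.
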(event Custom|OnCurrentUpdate_Event
  (params (Current :type Float%20%28double-precision%29))
  (Transformation|SetRelativeRotation (Variables|Default|GetDefaultSceneRoot) (Math|Rotator|MakeRotator 0.0 (* (/ Current (Variables|Default|GetOpenTime)) (Variables|Initial|GetRotateAngle)) 0.0) false false))

(event EventBeginPlay
  (EventDispatchers|AssignOnCurrentUpdate (Variables|Default|GetBP_DoorStopwatch) (delegate Custom|OnCurrentUpdate_Event)))

(fn ConstructionScript
  (Components|StaticMesh|SetStaticMesh (Variables|Default|GetStaticMesh) (Variables|Initial|GetMesh)))

(fn SetOpen
  (params (Openned :type Boolean))
  (if Openned
    (Default|Countto (Variables|Default|GetBP_DoorStopwatch) (Variables|Default|GetOpenTime))
    (else
      (Default|Countto (Variables|Default|GetBP_DoorStopwatch) 0.0))))