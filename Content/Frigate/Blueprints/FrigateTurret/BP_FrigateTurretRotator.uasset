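; Frigate turret rotator that turns a turret's yaw and pitch parts to follow a target actor's root component.
; Init supplies the turret wrapper and rotation interpolator, and SetTargetActor stores the actor's root component or clears the target.
; Each tick with a valid target, a shared rotation helper interpolates from the wrapper's world transforms toward the target location, and the wrapper applies the resulting rotations.
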(event EventTick
  (params (DeltaSeconds :type Float%20%28single-precision%29))
  (Private|TickTurretRotation))

(event EventBeginPlay
  (bind _instance (Utilities|GetorCreateTurretRotationHelper))
  (Variables|Default|SetTurretRotationHelper _instance)
  (bind _instance_2 (Utilities|GetorCreateMathHelper))
  (Variables|Default|SetMathHelpers _instance_2))

(fn Init
  (params (TurretWrapper :type BP%20Frigate%20Turret%20Wrapper%20Object%20Reference) (RotationInterpolator :type BPI%20Rotation%20Interpolator%20Interface))
  (Variables|Default|SetTurretWrapper TurretWrapper)
  (Variables|Default|SetRotation%20Interpolator RotationInterpolator))

(fn SetTargetActor
  (params (Target :type Actor%20Object%20Reference))
  (Utilities|IsValid Target
    (:Is%20Valid
      (Variables|Default|SetTarget (Variables|/Script/Engine.Actor|GetRootComponent Target)))
    (:Is%20Not%20Valid
      (Variables|Default|SetTarget 0))))

(fn TickTurretRotation
  (bind _turretwrapper (Variables|Default|GetTurretWrapper))
  (bind (_pitchworldtransform _yawworldtransform) (Default|GetTurretWorldTransform _turretwrapper))
  (bind (_location _rotation) (Math|Transform|BreakTransform _yawworldtransform))
  (bind (_location_2 _rotation_2) (Math|Transform|BreakTransform _pitchworldtransform))
  (Utilities|IsValid (Variables|Default|GetTarget)
    (:Is%20Valid
      (bind (_outpitchrotation _outyawrotation) (Default|InterpolateTurretRotationforTarget (Variables|Default|GetTurretRotationHelper) (Variables|Default|GetRotation%20Interpolator) _location_2 _rotation_2 _location _rotation (Transformation|GetWorldLocation (Variables|Default|GetTarget)) (Utilities|Time|GetWorldDeltaSeconds)))
      (Default|SetTurretRotation (Variables|Default|GetTurretWrapper) _outpitchrotation _outyawrotation))))