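; Frigate turret actor that assembles twin guns and bullet-drop particle effects and aims them at a target actor.
; On BeginPlay it casts its child actors to typed references, then attaches both guns and drops to the turret wrapper and passes shoot particles to the guns.
; A rotator component, initialized with an interpolator and pitch and yaw clamps, handles aiming.
; Shoot toggles both guns and pauses or resumes the bullet-drop particles accordingly.
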(event EventTick
  (params (DeltaSeconds :type Float%20%28single-precision%29)))

(event EventBeginPlay
  (Private|Unwrap)
  (Private|InitGuns)
  (Private|InitRotator))

(fn ConstructionScript)

(fn SetTarget
  (params (Target :type Actor%20Object%20Reference))
  (Default|SetTargetActor (Variables|Default|GetBP_FrigateTurretRotator) Target))

(fn Shoot
  (params (IsShooting :type Boolean))
  (bind _returnvalue (not IsShooting))
  (Default|Shoot (Variables|Default|GetLeftGun) IsShooting)
  (Default|Shoot (Variables|Default|GetRightGun) IsShooting)
  (Default|SetPaused (Variables|Default|GetLeftBulletDrop) _returnvalue)
  (Default|SetPaused (Variables|Default|GetRightBulletDrop) _returnvalue))

(fn Unwrap
  (Utilities|FlowControl|Sequence
    (:then_0
      (bind _asbp_frigate_turret_wrapper (Utilities|Casting|CastToBP_FrigateTurretWrapper (Variables|/Script/Engine.ChildActorComponent|GetChildActor (Variables|Default|GetCAC_TurretWrapper))))
      (Variables|Default|SetTurretWrapper _asbp_frigate_turret_wrapper))
    (:then_1
      (bind _asbp_frigate_turret_gun (Utilities|Casting|CastToBP_FrigateTurretGun (Variables|/Script/Engine.ChildActorComponent|GetChildActor (Variables|Default|GetCAC_LeftGun))))
      (Variables|Default|SetLeftGun _asbp_frigate_turret_gun))
    (:then_2
      (bind _asbp_frigate_turret_gun_2 (Utilities|Casting|CastToBP_FrigateTurretGun (Variables|/Script/Engine.ChildActorComponent|GetChildActor (Variables|Default|GetCAC_RightGun))))
      (Variables|Default|SetRightGun _asbp_frigate_turret_gun_2))
    (:then_3
      (bind _asbp_particles (Utilities|Casting|CastToBP_Particles (Variables|/Script/Engine.ChildActorComponent|GetChildActor (Variables|Default|GetCAC_LeftBulletDrop))))
      (Variables|Default|SetLeftBulletDrop _asbp_particles))
    (:then_4
      (bind _asbp_particles_2 (Utilities|Casting|CastToBP_Particles (Variables|/Script/Engine.ChildActorComponent|GetChildActor (Variables|Default|GetCAC_RightBulletDrop))))
      (Variables|Default|SetRightBulletDrop _asbp_particles_2))))

(fn InitRotator
  (bind _bp_frigateturretrotator (Variables|Default|GetBP_FrigateTurretRotator))
  (Default|Init _bp_frigateturretrotator (Variables|Default|GetTurretWrapper) (Variables|Default|GetBP_InterpRotatorInterpolator) (Variables|Initial|GetPitchClamp) (Variables|Initial|GetYawClamp))
  (Default|SetTargetActor _bp_frigateturretrotator (Variables|Initial|GetTargetActor)))

(fn InitGuns
  (bind _shootparticlesystem (Variables|Initial|GetShootParticleSystem))
  (bind _shootniagara (Variables|Initial|GetShootNiagara))
  (bind _turretwrapper (Variables|Default|GetTurretWrapper))
  (bind _turretwrapper_2 (Variables|Default|GetTurretWrapper))
  (Utilities|FlowControl|Sequence
    (:then_0
      ;[1 1 1] Guns Particles
      (Default|SetShootParticles (Variables|Default|GetLeftGun) _shootparticlesystem _shootniagara)
      (Default|SetShootParticles (Variables|Default|GetRightGun) _shootparticlesystem _shootniagara))
    (:then_1
      ;[1 1 1] Attach Guns
      (Default|AttachtoLeftGun _turretwrapper_2 (Variables|/Script/Engine.Actor|GetRootComponent (Variables|Default|GetLeftGun)) "KeepWorld")
      (Default|AttachtoRightGun _turretwrapper_2 (Variables|/Script/Engine.Actor|GetRootComponent (Variables|Default|GetRightGun)) "KeepWorld"))
    (:then_2
      ;[1 1 1] Attach bullet drops
      (Default|AttachtoLeftGun _turretwrapper (Variables|/Script/Engine.Actor|GetRootComponent (Variables|Default|GetLeftBulletDrop)) "KeepWorld")
      (Default|AttachtoRightGun _turretwrapper (Variables|/Script/Engine.Actor|GetRootComponent (Variables|Default|GetRightBulletDrop)) "KeepWorld"))))