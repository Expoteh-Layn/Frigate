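; Frigate turret gun Blueprint that handles the gun's shooting particle effect.
; The construction script caches a BP_Particles instance from a child actor component and applies the configured initial transform to that component.
; BeginPlay assigns the initial particle system and Niagara effect, then pauses it.
; Shoot toggles the pause to show firing, and SetShootParticles swaps both effect assets at runtime.
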(event EventBeginPlay
  (Default|SetParticles (Variables|Default|GetShootParticles) (Variables|Initial|GetShootParticleSystemInitial) (Variables|Initial|GetShootNiagaraInitial))
  (Default|SetPaused (Variables|Default|GetShootParticles) true))

(fn ConstructionScript
  (CallFunction|Unwrap)
  (Transformation|SetRelativeTransform (Variables|Default|GetShootParticlesComponent) (Variables|Initial|GetInitialShootTransform) false false))

(fn Shoot
  (params (IsShooting :type Boolean))
  (Default|SetPaused (Variables|Default|GetShootParticles) (not IsShooting)))

(fn SetShootParticles
  (params (ParticleSystem :type Particle%20System%20Object%20Reference) (Niagara :type Niagara%20System%20Object%20Reference))
  (Default|SetParticles (Variables|Default|GetShootParticles) ParticleSystem Niagara))

(fn Unwrap
  (Utilities|FlowControl|Sequence
    (:then_0
      (bind _asbp_particles (Utilities|Casting|CastToBP_Particles (Variables|/Script/Engine.ChildActorComponent|GetChildActor (Variables|Default|GetShootParticlesComponent))))
      (Variables|Default|SetShootParticles _asbp_particles))))