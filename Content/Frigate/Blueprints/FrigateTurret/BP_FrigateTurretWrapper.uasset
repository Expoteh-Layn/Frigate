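; Wrapper actor for the frigate turret that exposes rotation, transform and gun attachment functions.
; Yaw rotates the whole actor, while pitch is converted relative to yaw and passed to the ABP_FrigateTurret anim instance cached at BeginPlay.
; It reports yaw and pitch world transforms from the actor and TurretPitchSlave, and attaches components to the left or right gun slave components.
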(event EventBeginPlay
  (bind _asabp_frigate_turret (Utilities|Casting|CastToABP_FrigateTurret (Components|SkeletalMesh|GetAnimInstance (Variables|Default|GetSkeletalMesh))))
  (Variables|Default|SetAnimInstance _asabp_frigate_turret))

(fn ConstructionScript)

(fn SetTurretRotation
  (params (PitchRotation :type Rotator) (YawRotation :type Rotator))
  (Transformation|SetActorRotation YawRotation)
  (Default|SetTurretPitch (Variables|Default|GetAnimInstance) (.Pitch (Math|Rotator|BreakRotator (Default|ChildingRotation (Variables|Default|GetBP_MathHelpers) YawRotation PitchRotation)))))

(fn GetTurretWorldTransform
  (return (Transformation|GetWorldTransform (Variables|Default|GetTurretPitchSlave)) (Transformation|GetActorTransform)))

(fn AttachtoLeftGun
  (params (ComponentToBeAttached :type Scene%20Component%20Object%20Reference) (AttachRule :type EAttachmentRule%20Enum :default "SnapToTarget"))
  (Transformation|AttachComponentToComponent ComponentToBeAttached (Variables|Default|GetLeftGunSlave) "None" AttachRule AttachRule AttachRule true))

(fn AttachtoRightGun
  (params (ComponentToBeAttached :type Scene%20Component%20Object%20Reference) (AttachRule :type EAttachmentRule%20Enum :default "SnapToTarget"))
  (Transformation|AttachComponentToComponent ComponentToBeAttached (Variables|Default|GetRightGunSlave) "None" AttachRule AttachRule AttachRule true))