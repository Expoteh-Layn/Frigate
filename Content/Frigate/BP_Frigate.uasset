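; BP_Frigate is a ship driven by physics forces from forward and turn input values.
; Each Tick it adds force along the Frigate component's forward vector and yaw torque around Z, scaled by delta time.
; MoveForward and MoveRight store the input values, while two setters adjust speed multipliers that stack on separate core multipliers.
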(event EventTick
  (params (DeltaSeconds :type Float%20%28single-precision%29))
  (Utilities|FlowControl|Sequence
    (:then_0
      (Physics|AddForce (Variables|Default|GetFrigate) (* (Math|Vector|GetForwardVector (Variables|Default|GetFrigate)) (Variables|Default|GetForwardMultiCore) (Variables|Default|GetMoveForwardValue) DeltaSeconds (Variables|Default|GetForwardMulti)) "None" false))
    (:then_1
      (Class|PrimitiveComponent|AddTorqueinDegrees (Variables|Default|GetFrigate) (Math|Vector|MakeVector 0.0 0.0 (* (Variables|Default|GetMoveRightValue) (Variables|Default|GetRightMultiCore) (Variables|Default|GetRightMulti) DeltaSeconds)) "None" false))))

(fn ConstructionScript)

(fn MoveForward
  (params (value :type Float%20%28double-precision%29))
  (Variables|Default|SetMoveForwardValue value))

(fn MoveRight
  (params (Value :type Float%20%28double-precision%29))
  (Variables|Default|SetMoveRightValue Value))

(fn SetForwardSpeedMulti
  (params (value :type Float%20%28double-precision%29))
  (Variables|Default|SetForwardMulti value))

(fn SetRightSpeedMulti
  (params (value :type Float%20%28double-precision%29))
  (Variables|Default|SetRightMulti value))