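; Player camera controller for the frigate game that provides zoom and orbit controls over an assigned camera and spring arm.
; Setters supply the camera, spring arm and length range, and length changes are clamped to that range.
; Vertical input pitches the arm in local space while horizontal input yaws it in world space, with no pitch clamp.
; BeginPlay and Tick are unused, so external calls drive it.
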(event EventBeginPlay)

(event EventTick
  (params (DeltaSeconds :type Float%20%28single-precision%29)))

(fn SetCamera
  (params (Camera :type Camera%20Component%20Object%20Reference))
  (Variables|Default|SetCamera Camera))

(fn SetSpringArm
  (params (SpringArm :type Spring%20Arm%20Component%20Object%20Reference))
  (Utilities|FlowControl|Sequence
    (:then_0
      (Utilities|IsValid (Variables|Default|GetSpringArm)
        (:Is%20Valid
          (Variables|/Script/Engine.SpringArmComponent|SetTargetArmLength SpringArm (Variables|/Script/Engine.SpringArmComponent|GetTargetArmLength (Variables|Default|GetSpringArm))))))
    (:then_1
      (Variables|Default|SetSpringArm SpringArm))))

(fn SetLengthRange
  (params (MinLength :type Float%20%28double-precision%29) (MaxLength :type Float%20%28double-precision%29))
  (Variables|Default|SetLengthRange (Math|Vector2D|MakeVector2D MinLength MaxLength)))

(fn SetLength
  (params (Value :type Float%20%28double-precision%29))
  (bind _lengthrange (Variables|Default|GetLengthRange))
  (Variables|/Script/Engine.SpringArmComponent|SetTargetArmLength (Variables|Default|GetSpringArm) (Math|Float|Clamp(Float) Value (.x _lengthrange) (.y _lengthrange))))

(fn AddLength
  (params (Value :type Float%20%28double-precision%29))
  (CallFunction|SetLength (+ (Variables|/Script/Engine.SpringArmComponent|GetTargetArmLength (Variables|Default|GetSpringArm)) Value)))

(fn AddUp
  (params (Value :type Float%20%28double-precision%29))
  (Transformation|AddLocalRotation (Variables|Default|GetSpringArm) (Math|Rotator|MakeRotator 0.0 Value 0.0) false false))

(fn AddRight
  (params (Value :type Float%20%28double-precision%29))
  (Transformation|AddWorldRotation (Variables|Default|GetSpringArm) (Math|Rotator|MakeRotator 0.0 0.0 Value) false false))