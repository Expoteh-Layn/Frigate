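; BP_NiagaraParticlesBase is a base particle Blueprint that wraps a Niagara component with helpers for swapping and pausing its effect.
; Construction applies the initial pause state and Niagara system, and each swap resets override parameters and reapplies the stored pause state.
; Reset clears the asset, while Replicate copies the system from another particles instance rather than doing network replication.
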(fn ConstructionScript
  (CallFunction|SetPaused (Variables|Initial|GetIsPausedInitial))
  (CallFunction|SetParticles (Variables|Initial|GetNiagaraInitial)))

(fn SetParticles
  (params (Particles :type Niagara%20System%20Object%20Reference))
  (Class|NiagaraComponent|SetAsset (Variables|Default|GetNiagaraComponent) Particles true)
  (CallFunction|SetPaused (Variables|Initial|GetIsPausedInitial)))

(fn Reset
  (Class|NiagaraComponent|SetAsset (Variables|Default|GetNiagaraComponent) 0 true))

(fn SetPaused
  (params (IsPaused :type Boolean))
  (Variables|Initial|SetIsPausedInitial IsPaused)
  (Class|NiagaraComponent|SetPaused (Variables|Default|GetNiagaraComponent) IsPaused))

(fn Replicate
  (params (Particles :type BP%20Niagara%20Particles%20Base%20Object%20Reference))
  (CallFunction|SetParticles (AssetData|GetAsset (Variables|BP_NiagaraParticlesBase_C|GetNiagaraComponent Particles))))