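; BP_Particles is a helper that wraps a Cascade and a Niagara component so either kind of effect plays through one Blueprint.
; The construction script applies the paused state, then SetParticles, which gives a valid Cascade system priority over Niagara and resets both components before assigning the asset.
; SetPaused pauses or resumes Niagara directly, while for Cascade it toggles auto-activate and activates or deactivates the component.
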(event EventBeginPlay)

(fn ConstructionScript
  (CallFunction|SetPaused (Variables|Default|GetIsPaused))
  (CallFunction|SetParticles (Variables|Default|GetParticleSystem) (Variables|Default|GetNiagara)))

(fn SetParticles
  (params (ParticleSystem :type Particle%20System%20Object%20Reference) (Niagara :type Niagara%20System%20Object%20Reference))
  (Utilities|IsValid ParticleSystem
    (:Is%20Valid
      (CallFunction|Reset)
      (Effects|Components|ParticleSystem|SetTemplate (Variables|Default|GetParticleSystemComponent) ParticleSystem)
      (Variables|Default|SetParticleSystem ParticleSystem))
    (:Is%20Not%20Valid
      (Utilities|IsValid Niagara
        (:Is%20Valid
          (CallFunction|Reset)
          (Class|NiagaraComponent|SetAsset (Variables|Default|GetNiagaraComponent) Niagara true)
          (Variables|Default|SetNiagara Niagara))))))

(fn Reset
  (Effects|Components|ParticleSystem|SetTemplate (Variables|Default|GetParticleSystemComponent) 0)
  (Class|NiagaraComponent|SetAsset (Variables|Default|GetNiagaraComponent) 0 true)
  (Variables|Default|SetParticleSystem 0)
  (Variables|Default|SetNiagara 0))

(fn SetPaused
  (params (IsPaused :type Boolean))
  (bind _particlesystemcomponent (Variables|Default|GetParticleSystemComponent))
  (Variables|Default|SetIsPaused IsPaused)
  (Class|NiagaraComponent|SetPaused (Variables|Default|GetNiagaraComponent) IsPaused)
  (Components|Activation|SetAutoActivate _particlesystemcomponent (not IsPaused))
  (if IsPaused
    (Components|Activation|Deactivate _particlesystemcomponent)
    (else
      (Components|Activation|Activate _particlesystemcomponent false))))