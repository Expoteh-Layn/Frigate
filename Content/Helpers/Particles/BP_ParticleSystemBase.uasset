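; BP_ParticleSystemBase is a helper Blueprint that wraps a ParticleSystemComponent with a settable template and paused state.
; On BeginPlay it applies the initial paused state and template, and SetParticles stores any new template and reapplies that state.
; Pausing disables auto-activate and deactivates the component rather than freezing it.
; Replicate copies another instance's template rather than networking it, and Reset clears only the component's template.
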(event EventBeginPlay
  (CallFunction|SetPaused (Variables|Initial|GetIsPausedInitial))
  (CallFunction|SetParticles (Variables|Initial|GetParticleSystemInitial)))

(fn ConstructionScript)

(fn SetParticles
  (params (Particles :type Particle%20System%20Object%20Reference))
  (Variables|Initial|SetParticleSystemInitial Particles)
  (Effects|Components|ParticleSystem|SetTemplate (Variables|Default|GetParticleSystemComponent) Particles)
  (CallFunction|SetPaused (Variables|Initial|GetIsPausedInitial)))

(fn Reset
  (Effects|Components|ParticleSystem|SetTemplate (Variables|Default|GetParticleSystemComponent) 0))

(fn SetPaused
  (params (IsPaused :type Boolean))
  (bind _particlesystemcomponent (Variables|Default|GetParticleSystemComponent))
  (Variables|Initial|SetIsPausedInitial IsPaused)
  (Components|Activation|SetAutoActivate _particlesystemcomponent (not IsPaused))
  (if IsPaused
    (Components|Activation|Deactivate _particlesystemcomponent)
    (else
      (Components|Activation|Activate _particlesystemcomponent false))))

(fn IsPaused
  (return (Variables|Initial|GetIsPausedInitial)))

(fn Replicate
  (params (Particles :type BP%20Particle%20System%20Base%20Object%20Reference))
  (CallFunction|SetParticles (Variables|/Script/Engine.ParticleSystemComponent|GetTemplate (Variables|BP_ParticleSystemBase_C|GetParticleSystemComponent Particles))))