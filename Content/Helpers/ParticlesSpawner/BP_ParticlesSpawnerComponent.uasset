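; BP_ParticlesSpawnerComponent is a scene component that creates a Cascade or Niagara effect on its owning actor at BeginPlay, preferring Cascade when both are set.
; SetParticleSystem and SetNiagara each add a new component to the owner, assign the asset and snap-attach it to this component.
; Both call DestroyAll first, but it only checks validity and destroys nothing.
; Only the Cascade component reference is stored.
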(event EventBeginPlay
  (bind _particlesystem (Variables|Default|GetParticleSystem))
  (bind _niagara (Variables|Default|GetNiagara))
  (Utilities|IsValid _particlesystem
    (:Is%20Valid
      (CallFunction|SetParticleSystem _particlesystem))
    (:Is%20Not%20Valid
      (Utilities|IsValid _niagara
        (:Is%20Valid
          (CallFunction|SetNiagara _niagara))))))

(fn AttachtoMe
  (params (Component :type Scene%20Component%20Object%20Reference))
  (Transformation|DetachFromComponent Component "KeepRelative" "KeepRelative" "KeepRelative" true)
  (Transformation|AttachComponentToComponent Component self "None" "SnapToTarget" "SnapToTarget" "SnapToTarget" false))

(fn SetParticleSystem
  (params (ParticleSystem :type Particle%20System%20Object%20Reference))
  (CallFunction|DestroyAll)
  (bind _returnvalue (Game|AddComponentbyClass (Components|GetOwner) "/Script/Engine.ParticleSystemComponent" false))
  (Effects|Components|ParticleSystem|SetTemplate _returnvalue ParticleSystem)
  (Variables|Default|SetParticleSystemComponent _returnvalue)
  (CallFunction|AttachtoMe _returnvalue))

(fn DestroyAll
  (Utilities|FlowControl|Sequence
    (:then_0
      (Utilities|IsValid (Variables|Default|GetParticleSystemComponent)))
    (:then_1
      (Utilities|IsValid (Variables|Default|GetNiagaraComponent)))))

(fn SetNiagara
  (params (Niagara :type Niagara%20System%20Object%20Reference))
  (CallFunction|DestroyAll)
  (bind _returnvalue (Game|AddComponentbyClass (Components|GetOwner) "/Script/Niagara.NiagaraComponent" false))
  (Class|NiagaraComponent|SetAsset _returnvalue Niagara true)
  (CallFunction|AttachtoMe _returnvalue))