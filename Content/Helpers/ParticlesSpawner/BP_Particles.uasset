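; A helper actor that spawns either a Cascade particle system or a Niagara effect, chosen by which asset is set on it.
; The construction script applies the paused state, then a validity switch assigns the Cascade template first, otherwise the Niagara asset.
; Each setter clears both components before assigning, so only one effect plays at a time.
; Pausing pauses Niagara directly and toggles auto-activation and activation on the Cascade component.
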(event EventBeginPlay)

(fn ConstructionScript
  (CallFunction|SetPaused (Variables|Default|GetIsPaused))
  (Utilities|Switch
    (:ParticleSystem
      (CallFunction|SetParticleSystem (Variables|Default|GetParticleSystem)))
    (:Niagara
      (CallFunction|SetNiagara (Variables|Default|GetNiagara)))))

(fn SetParticleSystem
  (params (NewTemplate :type Particle%20System%20Object%20Reference))
  (CallFunction|ResetAll)
  (Effects|Components|ParticleSystem|SetTemplate (Variables|Default|GetParticleSystemComponent) NewTemplate)
  (Variables|Default|SetParticleSystem NewTemplate))

(fn SetNiagara
  (params (InAsset :type Niagara%20System%20Object%20Reference))
  (CallFunction|ResetAll)
  (Class|NiagaraComponent|SetAsset (Variables|Default|GetNiagaraComponent) InAsset true)
  (Variables|Default|SetNiagara InAsset))

(fn ResetAll
  (Effects|Components|ParticleSystem|SetTemplate (Variables|Default|GetParticleSystemComponent) 0)
  (Class|NiagaraComponent|SetAsset (Variables|Default|GetNiagaraComponent) 0 true)
  (Variables|Default|SetParticleSystem 0)
  (Variables|Default|SetNiagara 0))

(fn SetPaused
  (params (IsPaused :type Boolean))
  (bind _particlesystemcomponent (Variables|Default|GetParticleSystemComponent))
  (Variables|Default|SetIsPaused IsPaused)
  (Class|NiagaraComponent|SetPaused (Variables|Default|GetNiagaraComponent) IsPaused)
  (Components|Activation|SetAutoActivate _particlesystemcomponent (not IsPaused))
  (if IsPaused
    (Components|Activation|Deactivate _particlesystemcomponent)
    (else
      (Components|Activation|Activate _particlesystemcomponent false))))