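; Math helper library of small functions for rotator composition and vector flattening.
; Flat functions zero one vector axis, while local add, subtract and unchilding wrap CombineRotators, with subtraction negating the rotator first.
; ChildingRotation expresses a rotation relative to a parent through Unrotate, which unrotates the three axes and rebuilds a rotator from them.
; DeltaRotators reuses ChildingRotation to get the finish rotation relative to the start.
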(fn AddLocalRotation
  (params (Input :type Rotator) (AddRotation :type Rotator))
  (return (Math|Rotator|CombineRotators AddRotation Input)))

(fn SubtractLocalRotation
  (params (Input :type Rotator) (SubtractRotation :type Rotator))
  (return (Math|Rotator|CombineRotators (Class|KismetMathLibrary|NegateRotator SubtractRotation) Input)))

(fn FlatZ
  (params (Input :type Vector))
  (bind (_x _y) (Math|Vector|BreakVector Input))
  (return (Math|Vector|MakeVector _x _y 0.0)))

(fn FlatY
  (params (Input :type Vector))
  (bind (_x _y _z) (Math|Vector|BreakVector Input))
  (return (Math|Vector|MakeVector _x 0.0 _z)))

(fn FlatX
  (params (Input :type Vector))
  (bind (_x _y _z) (Math|Vector|BreakVector Input))
  (return (Math|Vector|MakeVector 0.0 _y _z)))

(fn ChildingRotation
  (params (ParentRotation :type Rotator) (RotationToMakeChild :type Rotator))
  (return (CallFunction|Unrotate RotationToMakeChild ParentRotation)))

(fn UnchildingRotation
  (params (ParentRotation :type Rotator) (ChildRotation :type Rotator))
  (return (Math|Rotator|CombineRotators ParentRotation ChildRotation)))

(fn DeltaRotators
  (params (StartRotator :type Rotator) (FinishRotator :type Rotator))
  (return (CallFunction|ChildingRotation StartRotator FinishRotator)))

(fn Unrotate
  (params (Input :type Rotator) (Unrotator :type Rotator))
  (bind (_x _y _z) (Math|Rotator|BreakRotIntoAxes Input))
  (return (Math|Rotator|MakeRotationfromAxes (Math|Vector|UnrotateVector _x Unrotator) (Math|Vector|UnrotateVector _y Unrotator) (Math|Vector|UnrotateVector _z Unrotator))))