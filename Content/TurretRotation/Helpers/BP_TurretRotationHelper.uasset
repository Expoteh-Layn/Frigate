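; Helper that computes aim rotations for a two-axis turret with separate yaw and pitch parts.
; Target yaw comes from the target direction flattened in the yaw part's local space, and pitch aims from the pivot using that yaw's right axis.
; Interpolation reduces current-to-target rotations to local pitch and yaw deltas, passes them through a supplied interpolator, then reapplies them as local rotations via a cached MathHelper.
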(event EventBeginPlay
  (bind _instance (Utilities|GetorCreateMathHelper))
  (Variables|Default|SetMath%20Helper _instance))

(fn GetTurretRotationforTarget
  (params (TurretPitchLocation :type Vector) (TurretYawRotation :type Rotator) (Target :type Vector))
  (bind _returnvalue (Math|Vector|MakeVector 0.0 0.0 1.0))
  (bind _returnvalue_2 (- Target TurretPitchLocation))
  (bind _math_helper (Variables|Default|GetMath%20Helper))
  (bind _math_helper_2 (Variables|Default|GetMath%20Helper))
  (bind _returnvalue_3 (Math|Vector|UnrotateVector _returnvalue_2 TurretYawRotation))
  (bind _output (Default|FlatZ _math_helper _returnvalue_3))
  (bind _returnvalue_4 (Math|Vector|Normalize _output))
  (bind _returnvalue_5 (Math|Rotator|MakeRotfromXZ _returnvalue_4 _returnvalue))
  (bind _yaw (Math|Rotator|BreakRotator _returnvalue_5))
  (bind _returnvalue_6 (Math|Rotator|MakeRotator 0.0 0.0 _yaw))
  (bind _output_2 (Default|AddLocalRotation _math_helper_2 TurretYawRotation _returnvalue_6))
  (return (Math|Rotator|MakeRotfromXY (Math|Vector|Normalize _returnvalue_2) (.Y (Math|Rotator|GetAxes _output_2))) _output_2))

(fn GetTurretLocalOffset
  (params (PitchStartRotation :type Rotator) (PitchFinishRotation :type Rotator) (YawStartRotation :type Rotator) (YawFinishRotation :type Rotator))
  (bind _math_helper (Variables|Default|GetMath%20Helper))
  (return (.Pitch (Math|Rotator|BreakRotator (Default|DeltaRotators _math_helper PitchStartRotation PitchFinishRotation))) (.Yaw (Math|Rotator|BreakRotator (Default|DeltaRotators _math_helper YawStartRotation YawFinishRotation)))))

(fn AddTurretLocalOffset
  (params (PitchInput :type Rotator) (YawInput :type Rotator) (PitchLocalOffset :type Float%20%28double-precision%29) (YawLocalOffset :type Float%20%28double-precision%29))
  (bind _math_helper (Variables|Default|GetMath%20Helper))
  (return (Default|AddLocalRotation _math_helper PitchInput (Math|Rotator|MakeRotator 0.0 PitchLocalOffset 0.0)) (Default|AddLocalRotation _math_helper YawInput (Math|Rotator|MakeRotator 0.0 0.0 YawLocalOffset))))

(fn InterpolateTurretRotationforTarget
  (params (RotatorInterpolator :type BPI%20Rotation%20Interpolator%20Interface) (PitchLocation :type Vector) (PitchRotation :type Rotator) (YawLocation :type Vector) (YawRotation :type Rotator) (Target :type Vector) (DeltaTime :type Float%20%28double-precision%29))
  (bind (_targetpitchrotation _targetyawrotation) (CallFunction|GetTurretRotationforTarget PitchLocation YawRotation Target))
  (bind (_interpolatedpitchrotation _interpolatedyawrotation _pitchlocaloffset _yawlocaloffset) (CallFunction|InterpolateTurretRotation PitchRotation _targetpitchrotation YawRotation _targetyawrotation RotatorInterpolator DeltaTime))
  (return _interpolatedpitchrotation _interpolatedyawrotation _pitchlocaloffset _yawlocaloffset))

(fn InterpolateTurretRotation
  (params (CurrentPitchRotation :type Rotator) (TargetPitchRotation :type Rotator) (CurrentYawRotation :type Rotator) (TargetYawRotation :type Rotator) (RotationInterpolator :type BPI%20Rotation%20Interpolator%20Interface) (DeltaTime :type Float%20%28double-precision%29))
  (bind (_pitchoffset _yawoffset) (CallFunction|GetTurretLocalOffset CurrentPitchRotation TargetPitchRotation CurrentYawRotation TargetYawRotation))
  (bind _output (Default|InterpolateRotation RotationInterpolator "0, 0, 0" (Math|Rotator|MakeRotator 0.0 _pitchoffset _yawoffset) DeltaTime))
  (return (.PitchOutput (CallFunction|AddTurretLocalOffset CurrentPitchRotation CurrentYawRotation (.Pitch (Math|Rotator|BreakRotator _output)) (.Yaw (Math|Rotator|BreakRotator _output)))) (.YawOutput (CallFunction|AddTurretLocalOffset CurrentPitchRotation CurrentYawRotation (.Pitch (Math|Rotator|BreakRotator _output)) (.Yaw (Math|Rotator|BreakRotator _output)))) (.Pitch (Math|Rotator|BreakRotator _output)) (.Yaw (Math|Rotator|BreakRotator _output))))