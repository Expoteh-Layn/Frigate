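; Helper Blueprint that computes pitch and yaw rotations for aiming a turret at a shoot position, using a MathHelper fetched on BeginPlay.
; Yaw comes from the target direction flattened in the yaw part's local space, so tilted turrets work.
; Pitch faces the target using the new yaw's right axis, and a wrapper accepts scene components.
; Two further functions extract and apply local pitch/yaw offsets between rotations.
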(event EventBeginPlay
  (bind _instance (Utilities|GetorCreateMathHelper))
  (Variables|Default|SetMath%20Helper _instance))

(fn TransformtoShootPosition
  (params (TurretPitchLocation :type Vector) (TurretYawRotation :type Rotator) (ShootPosition :type Vector))
  (bind _returnvalue (Math|Vector|MakeVector 0.0 0.0 1.0))
  (bind _returnvalue_2 (- ShootPosition TurretPitchLocation))
  (bind _math_helper (Variables|Default|GetMath%20Helper))
  (bind _math_helper_2 (Variables|Default|GetMath%20Helper))
  (bind _returnvalue_3 (Math|Vector|UnrotateVector _returnvalue_2 TurretYawRotation))
  (bind _output (Default|FlatZ _math_helper _returnvalue_3))
  (bind _returnvalue_4 (Math|Vector|Normalize _output))
  (bind _returnvalue_5 (Math|Rotator|MakeRotfromXZ _returnvalue_4 _returnvalue))
  (bind _yaw (Math|Rotator|BreakRotator _returnvalue_5))
  (bind _returnvalue_6 (Math|Rotator|MakeRotator 0.0 0.0 _yaw))
  (bind _output_2 (Default|AddLocalRotation _math_helper_2 TurretYawRotation _returnvalue_6))
  (return (Math|Rotator|MakeRotfromXY (Math|Vector|Normalize _returnvalue_2) (.Y (Math|Rotator|GetAxes _output_2))) _output_2 _yaw))

(fn TransformtoShootPositionComponent
  (params (TurretPitch :type Scene%20Component%20Object%20Reference) (TurretYaw :type Scene%20Component%20Object%20Reference) (ShootPosition :type Vector))
  (bind _returnvalue (Transformation|GetWorldLocation TurretPitch))
  (bind _returnvalue_2 (Transformation|GetWorldRotation TurretYaw))
  (bind (_outpitchrotation _outyawrotation) (CallFunction|TransformtoShootPosition _returnvalue _returnvalue_2 ShootPosition))
  (return _outpitchrotation _outyawrotation))

(fn GetTurretLocalOffset
  (params (PitchStartRotation :type Rotator) (PitchFinishRotation :type Rotator) (YawStartRotation :type Rotator) (YawFinishRotation :type Rotator))
  (bind _math_helper (Variables|Default|GetMath%20Helper))
  (return (.Pitch (Math|Rotator|BreakRotator (Default|DeltaRotators _math_helper PitchStartRotation PitchFinishRotation))) (.Yaw (Math|Rotator|BreakRotator (Default|DeltaRotators _math_helper YawStartRotation YawFinishRotation)))))

(fn AddTurretLocalOffset
  (params (PitchInput :type Rotator) (YawInput :type Rotator) (PitchLocalOffset :type Float%20%28double-precision%29) (YawLocalOffset :type Float%20%28double-precision%29))
  (bind _math_helper (Variables|Default|GetMath%20Helper))
  (return (Default|AddLocalRotation _math_helper PitchInput (Math|Rotator|MakeRotator 0.0 PitchLocalOffset 0.0)) (Default|AddLocalRotation _math_helper YawInput (Math|Rotator|MakeRotator 0.0 0.0 YawLocalOffset))))