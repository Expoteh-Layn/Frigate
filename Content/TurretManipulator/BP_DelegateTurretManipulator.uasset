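; Turret manipulator that rotates a turret's yaw and pitch toward a target or by queued rotation offsets, communicating through delegates.
; While either mode is active, Tick requests current rotations; the update functions compute and broadcast new ones.
; Target mode converts the shoot position into local offsets; Add mode consumes accumulated pitch/yaw, both smoothed by an injected RotatorsInterpolator.
; Setting a target clears queued offsets, and adding rotation clears the target.
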(event EventTick
  (params (DeltaSeconds :type Float%20%28single-precision%29))
  (Utilities|SwitchMode
    (:Target
      (Default|CallUpdateTurretCurrentRotations))
    (:Add
      (Default|CallUpdateTurretCurrentRotations))))

(event EventBeginPlay
  (bind _instance (Utilities|GetorCreateTurretRotationHelper))
  (Variables|Default|SetTurretHelper _instance)
  (bind _instance_2 (Utilities|GetorCreateMathHelper))
  (Variables|Default|SetMathHelper _instance_2))

(fn Init
  (params (RotatorsInterpolator :type BPI%20Rotatorterpolator%20Interface))
  (Variables|Default|SetRotatorsInterpolator RotatorsInterpolator))

(fn SetTarget
  (params (Target :type Scene%20Component%20Object%20Reference))
  (Private|ResetforTarget)
  (Variables|Default|SetTarget Target))

(fn ClearTarget
  (Variables|Default|SetTarget 0))

(fn UpdateTurretCurrentValues
  (params (PitchLocation :type Vector) (PitchRotation :type Rotator) (YawLocation :type Vector) (YawRotation :type Rotator))
  (Utilities|SwitchMode
    (:Target
      (Private|TickTarget PitchLocation PitchRotation YawRotation))
    (:Add
      (Private|TickAdd PitchRotation YawRotation))))

(fn UpdateTurretCurrentValues1
  (params (PitchLocation :type Vector) (PitchLocalRotation :type Float%20%28double-precision%29) (YawLocation :type Vector) (YawRotation :type Rotator))
  (Public|UpdateTurretCurrentValues PitchLocation (Default|UnchildingRotation (Variables|Default|GetMathHelper) YawRotation (Math|Rotator|MakeRotator 0.0 PitchLocalRotation 0.0)) YawLocation YawRotation))

(fn AddTurretRotation
  (params (Pitch :type Float%20%28double-precision%29) (Yaw :type Float%20%28double-precision%29))
  (Private|ResetforAdd)
  (Variables|Default|SetAddPitch (+ (Variables|Default|GetAddPitch) Pitch))
  (Variables|Default|SetAddYaw (+ (Variables|Default|GetAddYaw) Yaw)))

(fn IsAddMode
  (return (not (and (Math|Float|NearlyEqual(Float) (Variables|Default|GetAddPitch) 0.0 1e-06) (Math|Float|NearlyEqual(Float) (Variables|Default|GetAddYaw) 0.0 1e-06)))))

(fn IsTargetMode
  (return (Utilities|IsValid (Variables|Default|GetTarget))))

(fn TickTarget
  (params (PitchLocation :type Vector) (PitchRotation :type Rotator) (YawRotation :type Rotator))
  (bind _turrethelper (Variables|Default|GetTurretHelper))
  (bind _turrethelper_2 (Variables|Default|GetTurretHelper))
  (bind _target (Variables|Default|GetTarget))
  (bind _returnvalue (Transformation|GetWorldLocation _target))
  (bind (_outpitchrotation _outyawrotation) (Default|TransformtoShootPosition _turrethelper PitchLocation YawRotation _returnvalue))
  (bind (_pitchoffset _yawoffset) (Default|GetTurretLocalOffset _turrethelper_2 PitchRotation _outpitchrotation YawRotation _outyawrotation))
  (bind _output (Default|InterpolateRotation (Variables|Default|GetRotatorsInterpolator) "0, 0, 0" (Math|Rotator|MakeRotator 0.0 _pitchoffset _yawoffset) (Utilities|Time|GetWorldDeltaSeconds)))
  (Default|CallSetTurretRotations (.PitchOutput (Default|AddTurretLocalOffset (Variables|Default|GetTurretHelper) PitchRotation YawRotation (.Pitch (Math|Rotator|BreakRotator _output)) (.Yaw (Math|Rotator|BreakRotator _output)))) (.YawOutput (Default|AddTurretLocalOffset (Variables|Default|GetTurretHelper) PitchRotation YawRotation (.Pitch (Math|Rotator|BreakRotator _output)) (.Yaw (Math|Rotator|BreakRotator _output)))) (.pitch (Default|ChildingRotation (Variables|Default|GetMathHelper) (.YawOutput (Default|AddTurretLocalOffset (Variables|Default|GetTurretHelper) PitchRotation YawRotation (.Pitch (Math|Rotator|BreakRotator _output)) (.Yaw (Math|Rotator|BreakRotator _output)))) (.PitchOutput (Default|AddTurretLocalOffset (Variables|Default|GetTurretHelper) PitchRotation YawRotation (.Pitch (Math|Rotator|BreakRotator _output)) (.Yaw (Math|Rotator|BreakRotator _output)))))) (.Pitch (Math|Rotator|BreakRotator _output)) (.Yaw (Math|Rotator|BreakRotator _output))))

(fn TickAdd
  (params (PitchRotation :type Rotator) (YawRotation :type Rotator))
  (bind _output (Default|InterpolateRotation (Variables|Default|GetRotatorsInterpolator) "0, 0, 0" (Math|Rotator|MakeRotator 0.0 (Variables|Default|GetAddPitch) (Variables|Default|GetAddYaw)) (Utilities|Time|GetWorldDeltaSeconds)))
  (Variables|Default|SetAddPitch (- (Variables|Default|GetAddPitch) (.Pitch (Math|Rotator|BreakRotator _output))))
  (Variables|Default|SetAddYaw (- (Variables|Default|GetAddYaw) (.Yaw (Math|Rotator|BreakRotator _output))))
  (Default|CallSetTurretRotations (Default|AddLocalRotation (Variables|Default|GetMathHelper) PitchRotation (Math|Rotator|MakeRotator 0.0 (.Pitch (Math|Rotator|BreakRotator _output)) 0.0)) (Default|AddLocalRotation (Variables|Default|GetMathHelper) YawRotation (Math|Rotator|MakeRotator 0.0 0.0 (.Yaw (Math|Rotator|BreakRotator _output)))) (.pitch (Default|ChildingRotation (Variables|Default|GetMathHelper) (Default|AddLocalRotation (Variables|Default|GetMathHelper) YawRotation (Math|Rotator|MakeRotator 0.0 0.0 (.Yaw (Math|Rotator|BreakRotator _output)))) (Default|AddLocalRotation (Variables|Default|GetMathHelper) PitchRotation (Math|Rotator|MakeRotator 0.0 (.Pitch (Math|Rotator|BreakRotator _output)) 0.0)))) (.Pitch (Math|Rotator|BreakRotator _output)) (.Yaw (Math|Rotator|BreakRotator _output))))

(fn IsSetMode
  (return false))

(fn ResetforTarget
  (Variables|Default|SetAddPitch 0.0)
  (Variables|Default|SetAddYaw 0.0))

(fn ResetforAdd
  (Public|ClearTarget))