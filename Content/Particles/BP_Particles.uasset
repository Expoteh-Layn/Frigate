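; BP_Particles is a wrapper actor that exposes one interface for both Cascade and Niagara particle effects.
; Construction unwraps two child actors into typed references, then applies the initial pause state and effect assets.
; Setting particles resets both children and assigns only one effect, preferring a valid Cascade system over Niagara.
; Reset, pause and replicate calls forward to both children, with Replicate passing in the matching children of another particles instance.
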(event EventBeginPlay)

(fn ConstructionScript
  (CallFunction|Unwrap)
  (CallFunction|SetPaused (Variables|Initial|GetIsPausedInitial))
  (CallFunction|SetParticles (Variables|Initial|GetParticleSystemInitial) (Variables|Initial|GetNiagaraInitial)))

(fn SetParticles
  (params (ParticleSystem :type Particle%20System%20Object%20Reference) (Niagara :type Niagara%20System%20Object%20Reference))
  (CallFunction|Reset)
  (Utilities|IsValid ParticleSystem
    (:Is%20Valid
      (Default|SetParticles (Variables|Default|GetParticleSystem) ParticleSystem))
    (:Is%20Not%20Valid
      (Utilities|IsValid Niagara
        (:Is%20Valid
          (Default|SetParticles (Variables|Default|GetNiagara) Niagara))))))

(fn Reset
  (Default|Reset (Variables|Default|GetNiagara))
  (Default|Reset (Variables|Default|GetParticleSystem)))

(fn SetPaused
  (params (IsPaused :type Boolean))
  (Default|SetPaused (Variables|Default|GetNiagara) IsPaused)
  (Default|SetPaused (Variables|Default|GetParticleSystem) IsPaused))

(fn Replicate
  (params (Particles :type BP%20Particles%20Object%20Reference))
  (Default|Replicate (Variables|Default|GetNiagara) (Variables|BP_Particles_C|GetNiagara Particles))
  (Default|Replicate (Variables|Default|GetParticleSystem) (Variables|BP_Particles_C|GetParticleSystem Particles)))

(fn Unwrap
  (Utilities|FlowControl|Sequence
    (:then_0
      (bind _asbp_niagara_particles_base (Utilities|Casting|CastToBP_NiagaraParticlesBase (Variables|/Script/Engine.ChildActorComponent|GetChildActor (Variables|Default|GetCAC_Niagara))))
      (Variables|Default|SetNiagara _asbp_niagara_particles_base))
    (:then_1
      (bind _asbp_particle_system_base (Utilities|Casting|CastToBP_ParticleSystemBase (Variables|/Script/Engine.ChildActorComponent|GetChildActor (Variables|Default|GetCAC_ParticleSystem))))
      (Variables|Default|SetParticleSystem _asbp_particle_system_base))))