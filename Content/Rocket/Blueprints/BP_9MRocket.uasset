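; BP_9MRocket is a rocket actor with unfolding "flops", a particle engine effect and an explosion that destroys it.
; A stopwatch component counts toward the unwrap time or zero, and its updates drive flop rotation in the animation Blueprint as a normalized ratio.
; Prepare opens the flops, while Start also unpauses the engine's child-actor particles.
; Explode spawns a fireball emitter at the rocket's transform, then destroys the actor.
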(event Custom|OnCurrentUpdate_Event
  (params (Current :type Float%20%28double-precision%29))
  (Default|SetFlopsRotation (Variables|Default|GetAnimInstance) (/ Current (Variables|Default|GetFlopsUnwrapTime))))

(event EventBeginPlay
  (bind _asabp_9mrocket (Utilities|Casting|CastToABP_9MRocket (Components|SkeletalMesh|GetAnimInstance (Variables|Default|GetSkeletalMesh))))
  (Variables|Default|SetAnimInstance _asabp_9mrocket)
  (EventDispatchers|AssignOnCurrentUpdate (Variables|Default|GetBP_FlopsStopwatch) (delegate Custom|OnCurrentUpdate_Event))
  (bind _asbp_particles (Utilities|Casting|CastToBP_Particles (Variables|/Script/Engine.ChildActorComponent|GetChildActor (Variables|Default|GetEngine))))
  (Variables|Default|SetEngineParticles _asbp_particles))

(event EventExplode
  (bind _returnvalue (Transformation|GetActorTransform))
  (Effects|SpawnEmitteratLocation "/Game/ExplosionsMegaPack/Particles/ParticleEmitters/Fireballs/Fireballs_Large/Emitter_Fireball_Large_Radial_Var03_Medium.Emitter_Fireball_Large_Radial_Var03_Medium" (.location _returnvalue) (.rotation _returnvalue) (.scale _returnvalue))
  (Actor|DestroyActor))

(event EventStart
  (CallFunction|OpenFlops)
  (CallFunction|StartEngine))

(event EventTick
  (params (DeltaSeconds :type Float%20%28single-precision%29)))

(event EventPrepare
  (CallFunction|OpenFlops))

(fn ConstructionScript)

(fn OpenFlops
  (Default|Countto (Variables|Default|GetBP_FlopsStopwatch) (Variables|Default|GetFlopsUnwrapTime)))

(fn CloseFlops
  (Default|Countto (Variables|Default|GetBP_FlopsStopwatch) 0.0))

(fn StartEngine
  (Default|SetPaused (Variables|Default|GetEngineParticles) false))

(fn StopEngine
  (Default|SetPaused (Variables|Default|GetEngineParticles) true))

(fn GetRoot
  (return (Variables|Default|GetDefaultSceneRoot)))