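; A rocket actor that animates a rocket along two splines in sequence, a throw path and then a flight path, before exploding it.
; On BeginPlay it unwraps two spline mover child actors and the rocket child actor, then points each mover at the rocket's root and its spline.
; Start launches the throw; when it finishes, the fly spline detaches keeping its world transform and flight begins, ending in Explode.
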(event Custom|AnimationFinished_Event
  (Transformation|DetachFromComponent (Variables|Default|GetS_FlySpline) "KeepWorld" "KeepWorld" "KeepWorld" true)
  (Default|Start (Variables|Default|GetFlyAnimator)))

(event Custom|AnimationFinished_Event_0
  (Default|Explode (Variables|Default|GetRocket)))

(event EventBeginPlay
  (Private|Unwrap)
  (Private|ConfigureMover (Variables|Default|GetThrowAnimator) (Variables|Default|GetS_ThrowSpline))
  (Private|ConfigureMover (Variables|Default|GetFlyAnimator) (Variables|Default|GetS_FlySpline))
  (EventDispatchers|AssignAnimationFinished (Variables|Default|GetThrowAnimator) (delegate Custom|AnimationFinished_Event))
  (EventDispatchers|AssignAnimationFinished (Variables|Default|GetFlyAnimator) (delegate Custom|AnimationFinished_Event_0)))

(fn ConstructionScript)

(fn Unwrap
  (Utilities|FlowControl|Sequence
    (:then_0
      (bind _asbp_spline_mover (Utilities|Casting|CastToBP_SplineMover (Variables|/Script/Engine.ChildActorComponent|GetChildActor (Variables|Default|GetCAC_ThrowAnimator))))
      (Variables|Default|SetThrowAnimator _asbp_spline_mover))
    (:then_1
      (bind _asbp_spline_mover_2 (Utilities|Casting|CastToBP_SplineMover (Variables|/Script/Engine.ChildActorComponent|GetChildActor (Variables|Default|GetCAC_FlyAnimator))))
      (Variables|Default|SetFlyAnimator _asbp_spline_mover_2))
    (:then_2
      (bind _asbpi_rocket (Utilities|Casting|CastToBPI_Rocket (Variables|/Script/Engine.ChildActorComponent|GetChildActor (Variables|Default|GetCAC_Rocket))))
      (Variables|Default|SetRocket _asbpi_rocket))))

(fn ConfigureMover
  (params (Mover :type BP%20Spline%20Mover%20Object%20Reference) (Spline :type Spline%20Component%20Object%20Reference))
  (bind _root (Default|GetRoot (Variables|Default|GetRocket)))
  (Default|SetTarget Mover _root)
  (Default|SetSpline Mover Spline))

(fn Start
  (Default|Start (Variables|Default|GetThrowAnimator)))